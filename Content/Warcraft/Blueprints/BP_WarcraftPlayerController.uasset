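; Player controller that sets up input and the HUD for a Warcraft game player.
; On BeginPlay, for local controllers only, it adds the default and mouse-look Enhanced Input mapping contexts, then creates the W_PlayerHUD widget and adds it to the viewport.
; A ShouldUseTouchControls function always returns false.
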(event `self.ReceiveBeginPlay`
  ;[1 1 1] Initialize player input
  ;;[1 1 1] Only add input mappings to local players
  (if (`self.IsLocalPlayerController`)
    ;;[1 1 1] Add regular input mappings
    (`EnhancedInputSubsystemInterface.AddMappingContext` (subsystem `EnhancedInputLocalPlayerSubsystem`) "/Game/Input/IMC_Default.IMC_Default" 0 (struct))
    ;;[1 1 1] Add mouse look input mapping
    (`EnhancedInputSubsystemInterface.AddMappingContext` (subsystem `EnhancedInputLocalPlayerSubsystem`) "/Game/Input/IMC_MouseLook.IMC_MouseLook" 0 (struct))
    (bind _returnvalue (`|CreateWidget` "/Game/Warcraft/Widgets/W_PlayerHUD.W_PlayerHUD_C" self))
    (`UserWidget.AddToViewport` _returnvalue 0)))

(fn `Should Use Touch Controls`
  (returns (`Use Mobile Controls` :type Boolean))
  (return false))

(fn `UserConstructionScript`)